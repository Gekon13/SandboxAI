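; BP_TestCharacter is a test character that travels continuously along the spline of a referenced Spline actor.
; Each tick advances a distance by the movement component's MaxWalkSpeed, then sets location and rotation directly from the spline in world space.
; The location is raised by the capsule half-height along world up, and the distance wraps to zero at the spline's end.
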(event `self.ReceiveBeginPlay`
  (bind _distance (`self.distance`))
  (bind _splinecomponent (`SandboxAISplinePath.SplineComponent` (`self.spline`)))
  (set `self.distance` 0.0)
  (`self.K2_SetActorLocationAndRotation` (+ (`SplineComponent.GetLocationAtDistanceAlongSpline` _splinecomponent _distance "World") (* (`KismetMathLibrary.GetUpVector` (struct)) (`CapsuleComponent.GetScaledCapsuleHalfHeight` (`self.CapsuleComponent`)))) (`SplineComponent.GetRotationAtDistanceAlongSpline` _splinecomponent _distance "World") :!label _label)
  (if (<= (`SplineComponent.GetSplineLength` _splinecomponent) (`self.distance`))
    (set `self.distance` 0.0)))

(event `self.ReceiveTick`
  (params (DeltaSeconds :type "Float (single-precision)"))
  (set `self.distance` (+ (`self.distance`) (* DeltaSeconds (`CharacterMovementComponent.MaxWalkSpeed` (`self.CharacterMovement`)))))
  (goto _label))

(fn `UserConstructionScript`)